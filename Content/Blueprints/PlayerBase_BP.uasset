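; Base player Blueprint for a bomb-dropping game, handling force-driven movement, bomb placement and remote detonator pickup.
; MovePlayer applies mass-independent force to the Cube from calculated input.
; Overlapping a RemoteDetonator consumes it and grants detonator mode for a timed window.
; SpawnBombActor spawns an initialized bomb above the Cube, remote-styled in detonator mode; when spawning is refused in that mode, it destroys the player's own bombs.
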(event Collision|EventActorBeginOverlap
  (params (OtherActor :type Actor%20Object%20Reference))
  ;[1 1 1] Remote Detonator Pickup
  (bind _asremote_detonator (Utilities|Casting|CastToRemoteDetonator OtherActor))
  (Actor|DestroyActor _asremote_detonator)
  (Class|PlayerBase|DetonatorPicked)
  (Utilities|FlowControl|Delay 1e+01)
  (Class|PlayerBase|DetonatorExpired))

(fn ConstructionScript)

(fn MovePlayer
  (params (InputX :type Float%20%28single-precision%29) (InputY :type Float%20%28single-precision%29))
  (Physics|AddForce (Variables|Default|GetCube) (Class|PlayerBase|CalculateInputForce InputX InputY) "None" true))

(fn SpawnBombActor
  (bind _cube (Variables|Default|GetCube))
  (bind _hasdetonator (Variables|Default|GetHasDetonator))
  (bind _returnvalue (Transformation|GetWorldLocation _cube))
  (bind (_x _y _z) (Math|Vector|BreakVector _returnvalue))
  ;[1 1 1] Spawn Bomb
  (bind _returnvalue_2 (Class|PlayerBase|SpawnBomb))
  (if _returnvalue_2
    (bind _returnvalue_3 (Game|SpawnActorfromClass "/Game/Blueprints/BomB_Base.Bomb_Base_C" (Math|Conversions|ToTransform(Vector) (Math|Vector|MakeVector _x _y (+ _z 2e+02))) "Undefined" 0 0))
    (Class|Bomb|Initialize _returnvalue_3 self (Variables|Default|GetBlastMultiplier) _hasdetonator)
    (if _hasdetonator
      (Rendering|Material|SetMaterial (Variables|/Game/Blueprints/BomB_Base.Bomb_Base_C|GetSphere _returnvalue_3) 0 "/Game/Materials/RemoteBomb_MAT.RemoteBomb_MAT"))
    (else
      ;[1 1 1] Remote Detonator Case
      (if (Variables|Default|GetHasDetonator)
        (bind _outactors (Actor|GetAllActorsOfClass "/Game/Blueprints/BomB_Base.Bomb_Base_C"))
        (for _array_element _outactors
          (if (== (Variables|/Script/BombermanUE4.Bomb|GetSpawnedBy _array_element) self)
            (Actor|DestroyActor _array_element)))))))