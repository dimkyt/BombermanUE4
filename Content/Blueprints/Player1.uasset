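; Player 1 actor for a bomb-dropping game, with physics movement, bomb placement and a timed remote-detonator pickup.
; Tick pushes the Cube with acceleration-based force from the player's input axes, scaled by speed and multiplier.
; E spawns a Bomb1 above the Cube when SpawnBomb allows, passing blast and remote settings; otherwise, with a detonator, it destroys all Bomb1 actors.
; Overlapping a RemoteDetonator consumes it and grants the ability until a delayed expiry.
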(event Collision|EventActorBeginOverlap
  (params (OtherActor :type Actor%20Object%20Reference))
  ;[1 1 1] Remote Detonator Pickup
  (bind _asremote_detonator (Utilities|Casting|CastToRemoteDetonator OtherActor))
  (Actor|DestroyActor _asremote_detonator)
  (Class|PlayerBase|DetonatorPicked)
  (Utilities|FlowControl|Delay 1e+01)
  (Class|PlayerBase|DetonatorExpired))

(event EventTick
  (params (DeltaSeconds :type Float%20%28single-precision%29))
  (bind _speed (Variables|Default|GetSpeed))
  ;[1 1 1] Movement
  (Physics|AddForce (Variables|Default|GetCube) (* (Math|Vector|MakeVector (* (Input|AxisValues|GetUp_1) _speed) (* (Input|AxisValues|GetRight_1) _speed) 0.0) (Variables|Default|GetSpeedMultiplier)) "None" true))

(event Input|KeyboardEvents|E
  (params (Key :type Key%20Structure))
  (bind _cube (Variables|Default|GetCube))
  (bind _hasdetonator (Variables|Default|GetHasDetonator))
  (bind _returnvalue (Transformation|GetWorldLocation _cube))
  (bind (_x _y _z) (Math|Vector|BreakVector _returnvalue))
  ;[1 1 1] Spawn Bomb
  (:Pressed
    (bind _returnvalue_2 (Class|PlayerBase|SpawnBomb))
    (if _returnvalue_2
      (bind _returnvalue_3 (Game|SpawnActorfromClass "/Game/Blueprints/Bomb1.Bomb1_C" (Math|Conversions|ToTransform(Vector) (Math|Vector|MakeVector _x _y (+ _z 2e+02))) "Undefined" 0 0))
      (Class|Bomb|Initialize _returnvalue_3 (Variables|Default|GetBlastMultiplier) _hasdetonator)
      (if _hasdetonator
        (Rendering|Material|SetMaterial (Variables|/Game/Blueprints/Bomb1.Bomb1_C|GetSphere _returnvalue_3) 0 "/Game/Materials/RemoteBomb_MAT.RemoteBomb_MAT"))
      (else
        ;[1 1 1] Remote Detonator Case
        (if (Variables|Default|GetHasDetonator)
          (bind _outactors (Actor|GetAllActorsOfClass "/Game/Blueprints/Bomb1.Bomb1_C"))
          (for _array_element _outactors
            (Actor|DestroyActor _array_element)))))))

(fn ConstructionScript)