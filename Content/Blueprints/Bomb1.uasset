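; Timed bomb actor that destroys itself after BombDelay and blasts along four axis directions, in a cross shape.
; The blast runs in EndPlay, so any destruction of the bomb triggers it.
; For each Player1 actor, it calls BombDestroyed, then box-traces from the Sphere to each BlastEndpoint on the Visibility channel.
; Hit actors with CanBeDamaged set are destroyed outright, and the traces draw debug boxes.
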(event EventBeginPlay
  (Utilities|FlowControl|Delay (Variables|Default|GetBombDelay))
  (Actor|DestroyActor))

(event EventEndPlay
  (params (EndPlayReason :type EEndPlayReason%20Enum :default "Destroyed"))
  (bind _sphere (Variables|Default|GetSphere))
  (bind _returnvalue (Transformation|GetWorldLocation _sphere))
  ;[1 1 1] Destroy Bomb
  (bind _outactors (Actor|GetAllActorsOfClass "/Game/Blueprints/Player1.Player1_C"))
  (for _array_element _outactors
    (Class|PlayerBase|BombDestroyed _array_element)
    ;[1 1 1] Trace bomb blast
    (for _index (range 0 3)
      (bind _outhits (Class|KismetSystemLibrary|BoxTraceMulti _returnvalue (Class|Bomb|BlastEndpoint _returnvalue (Utilities|Select :Index _index :Option%200 "0.000000,-1.000000, 0" :Option%201 "0.000000,1.000000, 0" :Option%202 "1.000000, 0, 0" :Option%203 "-1.000000, 0, 0")) "20.000000,20.000000,20.000000" "0, 0, 0" "TraceTypeQuery1" false 0 "ForDuration" true))
      (for _array_element_2 _outhits
        (if (Variables|/Script/Engine.Actor|GetbCanBeDamaged (.HitActor (Collision|BreakHitResult _array_element_2)))
          (Actor|DestroyActor (.HitActor (Collision|BreakHitResult _array_element_2))))))))

(fn ConstructionScript)