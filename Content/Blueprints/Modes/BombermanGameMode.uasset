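; Game mode for a two-player Bomberman match that decides when a round ends and who won.
; Tick-driven Delays check Player1 and Player2 actor counts every quarter second and decrement a one-second countdown.
; Unequal counts set RoundState and increment the survivor's score in BombermanInstance; equal counts end the round only when both are gone or time expires.
; Ending a round pauses the game and shows EndRoundWidget.
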(event EventTick
  (params (DeltaSeconds :type Float%20%28single-precision%29))
  (bind _returnvalue (Game|GetGameInstance))
  (Utilities|FlowControl|Sequence
    (:then_0
      (Utilities|FlowControl|Delay 0.25)
      ;[1 1 1] Check player status and set round state
      (bind _outactors (Actor|GetAllActorsOfClass "/Game/Blueprints/Player1.Player1_C" :!label _label))
      (bind _outactors_2 (Actor|GetAllActorsOfClass "/Game/Blueprints/Player2.Player2_C"))
      (if (== (Utilities|Array|Length _outactors_2) (Utilities|Array|Length _outactors))
        (Variables|Default|SetRoundState "NewEnumerator1")
        (if (or (== (Utilities|Array|Length _outactors_2) 0) (<= (Variables|Default|GetSeconds) 0))
          ;[1 1 1] Pause game and display End Round screen
          (Game|SetGamePaused true :!label _label_2)
          (bind _returnvalue_2 (UserInterface|CreateWidget "/Game/Blueprints/UI/EndRoundWidget.EndRoundWidget_C"))
          (UserInterface|Viewport|AddtoViewport _returnvalue_2 0))
        (elif (< (Utilities|Array|Length _outactors_2) (Utilities|Array|Length _outactors))
          (Variables|Default|SetRoundState "NewEnumerator2")
          (bind _asbomberman_instance (Utilities|Casting|CastToBombermanInstance _returnvalue))
          (Math|Integer|IncrementInt (Variables|/Game/Blueprints/Modes/BombermanInstance.BombermanInstance_C|GetScorePlayer1 _asbomberman_instance)
            (:%20%20
              (goto _label_2)))
          (else
            (Variables|Default|SetRoundState "NewEnumerator3")
            (bind _asbomberman_instance_2 (Utilities|Casting|CastToBombermanInstance _returnvalue))
            (Math|Integer|IncrementInt (Variables|/Game/Blueprints/Modes/BombermanInstance.BombermanInstance_C|GetScorePlayer2 _asbomberman_instance_2)
              (:%20%20
                (goto _label_2)))))))
    (:then_1
      ;[1 1 1] Countdown Timer
      (Utilities|FlowControl|Delay 1.0)
      (bind _result (Math|Integer|DecrementInt (Variables|Default|GetSeconds))
        (:%20%20
          (if (<= _result 0)
            (goto _label)))))))

(fn ConstructionScript)