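; Game mode for a Bomberman game that runs the round countdown and decides the round's final state.
; Tick feeds a one-second Delay that decrements Seconds; at zero or below it pauses the game and shows the EndRoundWidget.
; It then sets RoundState to one of three values by comparing how many Player1 and Player2 actors remain.
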(event EventTick
  (params (DeltaSeconds :type Float%20%28single-precision%29))
  ;[1 1 1] Countdown Timer
  (Utilities|FlowControl|Delay 1.0)
  (bind _result (Math|Integer|DecrementInt (Variables|Default|GetSeconds))
    (:%20%20
      (if (<= _result 0)
        (Game|SetGamePaused true)
        (bind _returnvalue (UserInterface|CreateWidget "/Game/Blueprints/UI/EndRoundWidget.EndRoundWidget_C"))
        (UserInterface|Viewport|AddtoViewport _returnvalue 0)
        ;[1 1 1] Set final state of the round
        (bind _outactors (Actor|GetAllActorsOfClass "/Game/Blueprints/Player1.Player1_C"))
        (bind _outactors_2 (Actor|GetAllActorsOfClass "/Game/Blueprints/Player2.Player2_C"))
        (if (== (Utilities|Array|Length _outactors_2) (Utilities|Array|Length _outactors))
          (Variables|Default|SetRoundState "NewEnumerator1")
          (elif (< (Utilities|Array|Length _outactors_2) (Utilities|Array|Length _outactors))
            (Variables|Default|SetRoundState "NewEnumerator2")
            (else
              (Variables|Default|SetRoundState "NewEnumerator3"))))))))

(fn ConstructionScript)