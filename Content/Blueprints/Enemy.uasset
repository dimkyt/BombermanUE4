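; Enemy actor that wanders along the horizontal axes and destroys any PlayerBase actor it hits.
; BeginPlay picks a random direction from four axis-aligned options, and Tick moves the Cylinder component along it at constant speed using an unswept local offset.
; Hitting anything other than a PlayerBase picks a new random direction, which may repeat the current one.
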(event EventTick
  (params (DeltaSeconds :type Float%20%28single-precision%29))
  ;[1 1 1] Movement
  (Transformation|AddLocalOffset (Variables|Default|GetCylinder) (* (* (Variables|Default|GetDirection) DeltaSeconds) 5e+01) false false))

(event Collision|EventHit
  (params (MyComp :type Primitive%20Component%20Object%20Reference) (Other :type Actor%20Object%20Reference) (OtherComp :type Primitive%20Component%20Object%20Reference) (bSelfMoved :type Boolean) (HitLocation :type Vector :default "0, 0, 0") (HitNormal :type Vector :default "0, 0, 0") (NormalImpulse :type Vector :default "0, 0, 0") (Hit :type Hit%20Result%20Structure%20%28by%20ref%29))
  ;[1 1 1] Handle hits
  (bind _asplayer_base (Utilities|Casting|CastToPlayerBase Other)
    (:then
      (Actor|DestroyActor _asplayer_base))
    (:CastFailed
      (Variables|Default|SetDirection (Utilities|Select :Index (Math|Random|RandomIntegerinRange 0 3) :Option%200 "1.000000,0.000000,0.000000" :Option%201 "-1.000000, 0, 0" :Option%202 "0,1.000000,0.000000" :Option%203 "0.000000,-1.000000, 0")))))

(event EventBeginPlay
  ;[1 1 1] Set initial direction
  (Variables|Default|SetDirection (Utilities|Select :Index (Math|Random|RandomIntegerinRange 0 3) :Option%200 "1.000000,0.000000,0.000000" :Option%201 "-1.000000, 0, 0" :Option%202 "0,1.000000,0.000000" :Option%203 "0.000000,-1.000000, 0")))

(fn ConstructionScript)